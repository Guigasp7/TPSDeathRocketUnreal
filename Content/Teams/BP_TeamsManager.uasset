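; Teams manager Blueprint that colors each player's text render, likely the pseudo (name) label, by team.
; The SetPseudos event loops over the Players array from index zero through the supplied Nums, inclusive, and checks each player's TeamTag.
; Players tagged "Team 1" get red text on their TextRenderComponent, and all others get blue.
; It changes only the color, leaving the text itself untouched.
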(event EventSetPseudos
  (params (nums :type Integer))
  ;[1 1 1] Set Pseudos
  (for _index (range 0 nums)
    (if (Utilities|Enum|Equal(Enum) (Variables|/Script/DeathRocket_TPS.MyPlayer|GetteamTag (Utilities|Array|Get(acopy) (Variables|Default|Getplayers) _index)) "Team 1")
      (Rendering|Components|TextRender|SetTextRenderColor (Actor|GetComponentbyClass (Utilities|Array|Get(acopy) (Variables|Default|Getplayers) _index) "/Script/Engine.TextRenderComponent") (Math|Color|MakeColor 3 0 251 1))
      (else
        (Rendering|Components|TextRender|SetTextRenderColor (Actor|GetComponentbyClass (Utilities|Array|Get(acopy) (Variables|Default|Getplayers) _index) "/Script/Engine.TextRenderComponent") (Math|Color|MakeColor 255 0 0 1))))))