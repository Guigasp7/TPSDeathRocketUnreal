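; Game mode for a two-team multiplayer fighting game that handles character selection, match start and results.
; It creates the TeamsManager, and per-character events set the chosen player's mesh and ultimate ID and play a voice line.
; LaunchTimer counts ready players, then shows a timer widget, enables each player's input and HUD, and flags the game as running.
; Draw and team-win events clear all widgets and display the matching result screen.
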(event Custom|LaunchTimer
  (bind _teamsmanager (Variables|Default|GetTeamsManager))
  (bind _players (Variables|/Script/DeathRocket_TPS.TeamsManager|Getplayers _teamsmanager))
  (bind _returnvalue (Utilities|Array|Length _players))
  ;[1 1 1] Event Launch Game
  (bind _result (Math|Integer|IncrementInt (Variables|/Script/DeathRocket_TPS.TeamsManager|GetreadyPlayers (Variables|Default|GetTeamsManager)))
    (:%20%20
      (bind _output_get (Variables|/Script/DeathRocket_TPS.TeamsManager|SetreadyPlayers (Variables|Default|GetTeamsManager) _result))
      (if (>= _output_get _returnvalue)
        (bind _returnvalue_2 (UserInterface|CreateWidget "/Game/HUD/WBP_Timer.WBP_Timer_C"))
        (UserInterface|Viewport|AddtoViewport _returnvalue_2 0)
        (for _index (range 0 _returnvalue)
          (bind _asbp_player (Utilities|Casting|CastToBP_Player (Utilities|Array|Get(acopy) _players _index)))
          (bind _asplayer_controller (Utilities|Casting|CastToPlayerController (Pawn|GetController _asbp_player)))
          (Input|EnableInput _asbp_player _asplayer_controller)
          (Default|HudReady _asbp_player)
          (Audio|PlaySound2D "/Game/Assets/Sounds/MrHappy_Announcer/wav/24_Fight.24_Fight" 1.0 1.0 0.0 0 0)
          (Utilities|FlowControl|Delay 0.5)
          (Variables|Default|SetIsInGame true))))))

(event Custom|ChooseKachuijin
  (params (Id :type Integer))
  ;[1 1 1] Choose Kachuijin
  (bind _asbp_player (Utilities|Casting|CastToBP_Player (Pawn|GetControlledPawn (Game|GetPlayerController Id))))
  (Variables|/Script/DeathRocket_TPS.MyPlayer|SetultiId _asbp_player 2)
  (Variables|/Script/Engine.SkeletalMeshComponent|SetSkeletalMeshAsset (Variables|/Script/Engine.Character|GetMesh _asbp_player) "/Game/Player/Models/Kachujin_G_Rosales.Kachujin_G_Rosales")
  (Audio|PlaySoundatLocation "/Game/Assets/Sounds/TheAlertedNPC_Male/wav/03_Hey.03_Hey" (Transformation|GetActorLocation) "0, 0, 0" 1.0 1.0 0.0 0 0 0 0))

(event Custom|ChooseYBot
  (params (Id :type Integer))
  ;[1 1 1] Choose Y Bot
  (bind _asbp_player (Utilities|Casting|CastToBP_Player (Pawn|GetControlledPawn (Game|GetPlayerController Id))))
  (Variables|/Script/DeathRocket_TPS.MyPlayer|SetultiId _asbp_player 0)
  (Variables|/Script/Engine.SkeletalMeshComponent|SetSkeletalMeshAsset (Variables|/Script/Engine.Character|GetMesh _asbp_player) "/Game/Player/Models/Y_Bot.Y_Bot")
  (Audio|PlaySoundatLocation "/Game/Assets/Sounds/UrokTheOrc/wav/07_Do_Not_Test_My_Patience.07_Do_Not_Test_My_Patience" (Transformation|GetActorLocation _asbp_player) "0, 0, 0" 1.0 1.0 0.0 0 0 0 0))

(event Custom|ChooseCH48
  (params (Id :type Integer))
  ;[1 1 1] Choose CH48
  (bind _asbp_player (Utilities|Casting|CastToBP_Player (Pawn|GetControlledPawn (Game|GetPlayerController Id))))
  (Variables|/Script/DeathRocket_TPS.MyPlayer|SetultiId _asbp_player 0)
  (Variables|/Script/Engine.SkeletalMeshComponent|SetSkeletalMeshAsset (Variables|/Script/Engine.Character|GetMesh _asbp_player) "/Game/Player/Models/Ch48_nonPBR.Ch48_nonPBR")
  (Audio|PlaySoundatLocation "/Game/Assets/Sounds/UrokTheOrc/cues/14_You_Look_Weak_Cue.14_You_Look_Weak_Cue" (Transformation|GetActorLocation _asbp_player) "0, 0, 0" 1.0 1.0 0.0 0 0 0 0))

(event Custom|ChooseGaunfaul
  (params (Id :type Integer))
  ;[1 1 1] Choose Gaunfaul
  (bind _asbp_player (Utilities|Casting|CastToBP_Player (Pawn|GetControlledPawn (Game|GetPlayerController Id))))
  (Variables|/Script/DeathRocket_TPS.MyPlayer|SetultiId _asbp_player 1)
  (Variables|/Script/Engine.SkeletalMeshComponent|SetSkeletalMeshAsset (Variables|/Script/Engine.Character|GetMesh _asbp_player) "/Game/Player/Models/Ganfaul_M_Aure.Ganfaul_M_Aure")
  (Audio|PlaySoundatLocation "/Game/Assets/Sounds/UrokTheOrc/cues/19_Ha_ha_ha_ha_ha_Cue.19_Ha_ha_ha_ha_ha_Cue" (Transformation|GetActorLocation _asbp_player) "0, 0, 0" 1.0 1.0 0.0 0 0 0 0))

(event EventBeginPlay
  ;[1 1 1] Set TeamsManager
  (bind _returnvalue (Game|ConstructObjectfromClass "/Game/Teams/BP_TeamsManager.BP_TeamsManager_C"))
  (Variables|Default|SetTeamsManager _returnvalue))

(event EventSecondTeamWin
  ;[1 1 1] Team 2 win result
  (Viewport|RemoveAllWidgets)
  (bind _returnvalue (UserInterface|CreateWidget "/Game/HUD/WBP_Team2Win.WBP_Team2Win_C"))
  (bind _output_get (Variables|Default|SetWBP_Team2Win _returnvalue))
  (UserInterface|Viewport|AddtoViewport _output_get 0))

(event EventDraw
  ;[1 1 1] Draw Result
  (Viewport|RemoveAllWidgets)
  (bind _returnvalue (UserInterface|CreateWidget "/Game/HUD/WBP_Draw.WBP_Draw_C"))
  (bind _output_get (Variables|Default|SetWBP_Draw _returnvalue))
  (UserInterface|Viewport|AddtoViewport _output_get 0))

(event EventFirstTeamWin
  ;[1 1 1] Team 1 win result
  (Viewport|RemoveAllWidgets)
  (bind _returnvalue (UserInterface|CreateWidget "/Game/HUD/WBP_Team1Win.WBP_Team1Win_C" (Game|GetPlayerController 0)))
  (bind _output_get (Variables|Default|SetWBP_Team1Win _returnvalue))
  (UserInterface|Viewport|AddtoViewport _output_get 0))

(fn ConstructionScript)