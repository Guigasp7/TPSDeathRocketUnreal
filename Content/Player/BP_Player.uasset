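; BP_Player is the player pawn Blueprint, handling per-player UI, pausing and visual effects.
; It caches the game mode and TeamsManager, starts with input disabled, and uses PlayerIndex to give each local player selection, HUD and hold-to-show scoreboard widgets.
; The Start input opens a pause menu for player 0 during a match.
; Custom events toggle the grappling cable and the ultimate's Niagara and outline overlay effects.
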(event Custom|HudReady
  ;[1 1 1] Ready
  (Widget|RemovefromParent (Variables|Default|GetReadyHUD))
  (bind _returnvalue (UserInterface|CreateWidget "/Game/HUD/WBP_Player.WBP_Player_C" (Game|GetPlayerController (Variables|Default|GetplayerIndex))))
  (bind _output_get (Variables|Default|SetPlayerHud _returnvalue))
  (UserInterface|Viewport|AddtoPlayerScreen _output_get)
  (Input|SetInputModeGameOnly (Game|GetPlayerController (Variables|Default|GetplayerIndex)) false))

(event Input|EnhancedActionEvents|EnhancedInputActionIA_Start
  (params (ActionValue :type Boolean) (ElapsedSeconds :type Float%20%28double-precision%29) (TriggeredSeconds :type Float%20%28double-precision%29) (InputAction :type Input%20Action%20Object%20Reference :default "/Game/Player/Inputs/Actions/IA_Start.IA_Start"))
  ;[1 1 1] Pause
  (if (Variables|/Game/GameModes/BP_GameMode.BP_Gamemode_C|GetIsInGame (Variables|Default|GetAs%20BP%20Gamemode))
    (if (not (Variables|/Game/GameModes/BP_GameMode.BP_Gamemode_C|GetIsPaused (Variables|Default|GetAs%20BP%20Gamemode)))
      (bind _returnvalue (UserInterface|CreateWidget "/Game/HUD/WBP_MenuPause.WBP_MenuPause_C" (Game|GetPlayerController 0)))
      (bind _output_get (Variables|/Game/GameModes/BP_GameMode.BP_Gamemode_C|SetMenuPause (Variables|Default|GetAs%20BP%20Gamemode) _returnvalue))
      (UserInterface|Viewport|AddtoViewport _output_get 0)
      (Game|SetGamePaused true)
      (Input|SetInputModeGameandUI (Game|GetPlayerController 0) (Variables|/Game/HUD/WBP_MenuPause.WBP_MenuPause_C|GetResume _output_get) "DoNotLock" true false)
      (Variables|/Game/GameModes/BP_GameMode.BP_Gamemode_C|SetIsPaused (Variables|Default|GetAs%20BP%20Gamemode) false))))

(event Input|EnhancedActionEvents|EnhancedInputActionIA_ScoreBoard
  (params (ActionValue :type Boolean) (ElapsedSeconds :type Float%20%28double-precision%29) (TriggeredSeconds :type Float%20%28double-precision%29) (InputAction :type Input%20Action%20Object%20Reference :default "/Game/Player/Inputs/Actions/IA_ScoreBoard.IA_ScoreBoard"))
  ;[1 1 1] Show / Hide ScoreBoard
  (:Started
    (bind _returnvalue (UserInterface|CreateWidget "/Game/HUD/WBP_ScoreBoard.WBP_ScoreBoard_C" (Game|GetPlayerController (Variables|Default|GetplayerIndex))))
    (bind _output_get (Variables|Default|SetScoreBoardHud _returnvalue))
    (UserInterface|Viewport|AddtoPlayerScreen _output_get))
  (:Completed
    (Widget|RemovefromParent (Variables|Default|GetScoreBoardHud))))

(event EventBeginPlay
  ;[1 1 1] Begin Play
  (bind _asbp_gamemode (Utilities|Casting|CastToBP_Gamemode (Game|GetGameMode)))
  (bind _output_get (Variables|Default|SetAs%20BP%20Gamemode _asbp_gamemode))
  (Utilities|FlowControl|Delay 0.5)
  (Variables|Default|SetteamsManager (Variables|/Game/GameModes/BP_GameMode.BP_Gamemode_C|GetTeamsManager _output_get))
  (Input|DisableInput 0))

(event EventEnableUltimEffect
  ;[1 1 1] Enable/Disable Ultime Particules
  (Transformation|SetWorldScale3D (Variables|Default|GetniagaraComponent) "1.000000,1.000000,1.000000")
  (Rendering|Material|SetOverlayMaterial (Variables|Character|GetMesh) "/Game/Assets/Particles/FX/PlayerUltimeVFX/M_UltimeOutline.M_UltimeOutline" :!class /Script/Engine.MeshComponent))

(event EventAddHUDSelect
  (bind _playerindex (Variables|Default|GetplayerIndex))
  (bind _returnvalue (Game|GetPlayerController _playerindex))
  ;[1 1 1] HUD Choose Player add
  (bind _returnvalue_2 (UserInterface|CreateWidget "/Game/HUD/WBP_ChoosePlayer.WBP_ChoosePlayer_C" _returnvalue))
  (Input|SetInputModeGameandUI _returnvalue _returnvalue_2 "DoNotLock" true false)
  (bind _output_get (Variables|Default|SetSelectPlayer _returnvalue_2))
  (Variables|/Game/HUD/WBP_ChoosePlayer.WBP_ChoosePlayer_C|SetPlayerRef _output_get self)
  (UserInterface|Viewport|AddtoPlayerScreen _output_get))

(event EventDisableUltimEffect
  ;[1 1 1] Enable/Disable Ultime Particules
  (Transformation|SetWorldScale3D (Variables|Default|GetniagaraComponent) "0, 0, 0")
  (Rendering|Material|SetOverlayMaterial (Variables|Character|GetMesh) 0 :!class /Script/Engine.MeshComponent))

(event EventDrawGrapplingCable
  (bind _cable (Variables|Default|GetCable))
  ;[1 1 1] Draw and hide grappling hook
  (Variables|/Script/CableComponent.CableComponent|SetEndLocation _cable (Math|Transform|InverseTransformLocation (Transformation|GetActorTransform) (Variables|Default|GetgrapplingHitPoint)))
  (Rendering|SetVisibility _cable true false))

(event EventHideGrapplingCable
  ;[1 1 1] Draw and hide grappling hook
  (Rendering|SetVisibility (Variables|Default|GetCable) false false))

(fn ConstructionScript)