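; BP_Bird is an interactible actor that destroys itself when anything begins overlapping its Box1 component.
; After the destroy call, it casts player 0's pawn to BP_Player without checking the overlapping actor.
; It increments its own IncreaseScoreValue and assigns the result to PlayerScore, overwriting rather than adding to the score.
; It then hides Cube and disables collision on Cube and Box1.
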(event OnComponentBeginOverlap(Box1)
  (params (OverlappedComponent :type Primitive%20Component%20Object%20Reference) (OtherActor :type Actor%20Object%20Reference) (OtherComp :type Primitive%20Component%20Object%20Reference) (OtherBodyIndex :type Integer) (bFromSweep :type Boolean) (SweepResult :type Hit%20Result%20Structure%20%28by%20ref%29))
  (Actor|DestroyActor)
  (bind _asbp_player (Utilities|Casting|CastToBP_Player (Pawn|GetControlledPawn (Game|GetPlayerController 0))))
  (bind _result (Math|Integer|IncrementInt (Variables|Default|GetIncreaseScoreValue))
    (:%20%20
      (Variables|/Script/DeathRocket_TPS.MyPlayer|SetplayerScore _asbp_player _result)
      (Rendering|SetVisibility (Variables|Default|GetCube) false false)
      (Collision|SetCollisionEnabled (Variables|Default|GetCube) "NoCollision"))))

(fn ConstructionScript)