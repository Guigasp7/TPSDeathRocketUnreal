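; BP_Wheel is an interactible wheel with eight targets that Rocket actors knock out individually.
; Tick rotates component E by a fixed step each frame, so spin speed depends on frame rate.
; Eight box triggers each cast the overlapping actor to Rocket, then destroy their own paired R and Cube components.
; The trigger boxes themselves are never destroyed, and no score or completion state is tracked.
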(event OnComponentBeginOverlap(Box)
  (params (OverlappedComponent :type Primitive%20Component%20Object%20Reference) (OtherActor :type Actor%20Object%20Reference) (OtherComp :type Primitive%20Component%20Object%20Reference) (OtherBodyIndex :type Integer) (bFromSweep :type Boolean) (SweepResult :type Hit%20Result%20Structure%20%28by%20ref%29))
  (Utilities|Casting|CastToRocket OtherActor)
  (Components|DestroyComponent (Variables|Default|Getr))
  (Components|DestroyComponent (Variables|Default|GetCube)))

(event OnComponentBeginOverlap(Box7)
  (params (OverlappedComponent :type Primitive%20Component%20Object%20Reference) (OtherActor :type Actor%20Object%20Reference) (OtherComp :type Primitive%20Component%20Object%20Reference) (OtherBodyIndex :type Integer) (bFromSweep :type Boolean) (SweepResult :type Hit%20Result%20Structure%20%28by%20ref%29))
  (Utilities|Casting|CastToRocket OtherActor)
  (Components|DestroyComponent (Variables|Default|Getr3))
  (Components|DestroyComponent (Variables|Default|GetCube3)))

(event OnComponentBeginOverlap(Box6)
  (params (OverlappedComponent :type Primitive%20Component%20Object%20Reference) (OtherActor :type Actor%20Object%20Reference) (OtherComp :type Primitive%20Component%20Object%20Reference) (OtherBodyIndex :type Integer) (bFromSweep :type Boolean) (SweepResult :type Hit%20Result%20Structure%20%28by%20ref%29))
  (Utilities|Casting|CastToRocket OtherActor)
  (Components|DestroyComponent (Variables|Default|Getr2))
  (Components|DestroyComponent (Variables|Default|GetCube2)))

(event OnComponentBeginOverlap(Box2)
  (params (OverlappedComponent :type Primitive%20Component%20Object%20Reference) (OtherActor :type Actor%20Object%20Reference) (OtherComp :type Primitive%20Component%20Object%20Reference) (OtherBodyIndex :type Integer) (bFromSweep :type Boolean) (SweepResult :type Hit%20Result%20Structure%20%28by%20ref%29))
  (Utilities|Casting|CastToRocket OtherActor)
  (Components|DestroyComponent (Variables|Default|Getr5))
  (Components|DestroyComponent (Variables|Default|GetCube6)))

(event OnComponentBeginOverlap(Box1)
  (params (OverlappedComponent :type Primitive%20Component%20Object%20Reference) (OtherActor :type Actor%20Object%20Reference) (OtherComp :type Primitive%20Component%20Object%20Reference) (OtherBodyIndex :type Integer) (bFromSweep :type Boolean) (SweepResult :type Hit%20Result%20Structure%20%28by%20ref%29))
  (Utilities|Casting|CastToRocket OtherActor)
  (Components|DestroyComponent (Variables|Default|Getr6))
  (Components|DestroyComponent (Variables|Default|GetCube7)))

(event OnComponentBeginOverlap(Box4)
  (params (OverlappedComponent :type Primitive%20Component%20Object%20Reference) (OtherActor :type Actor%20Object%20Reference) (OtherComp :type Primitive%20Component%20Object%20Reference) (OtherBodyIndex :type Integer) (bFromSweep :type Boolean) (SweepResult :type Hit%20Result%20Structure%20%28by%20ref%29))
  (Utilities|Casting|CastToRocket OtherActor)
  (Components|DestroyComponent (Variables|Default|Getr1))
  (Components|DestroyComponent (Variables|Default|GetCube1)))

(event OnComponentBeginOverlap(Box3)
  (params (OverlappedComponent :type Primitive%20Component%20Object%20Reference) (OtherActor :type Actor%20Object%20Reference) (OtherComp :type Primitive%20Component%20Object%20Reference) (OtherBodyIndex :type Integer) (bFromSweep :type Boolean) (SweepResult :type Hit%20Result%20Structure%20%28by%20ref%29))
  (Utilities|Casting|CastToRocket OtherActor)
  (Components|DestroyComponent (Variables|Default|Getr7))
  (Components|DestroyComponent (Variables|Default|GetCube8)))

(event OnComponentBeginOverlap(Box5)
  (params (OverlappedComponent :type Primitive%20Component%20Object%20Reference) (OtherActor :type Actor%20Object%20Reference) (OtherComp :type Primitive%20Component%20Object%20Reference) (OtherBodyIndex :type Integer) (bFromSweep :type Boolean) (SweepResult :type Hit%20Result%20Structure%20%28by%20ref%29))
  (Utilities|Casting|CastToRocket OtherActor)
  (Components|DestroyComponent (Variables|Default|Getr4))
  (Components|DestroyComponent (Variables|Default|GetCube5)))

(event EventTick
  (params (DeltaSeconds :type Float%20%28single-precision%29))
  (Transformation|AddRelativeRotation (Variables|Default|Gete) "0.000000,3.000000,0.000000" false false))

(fn ConstructionScript)