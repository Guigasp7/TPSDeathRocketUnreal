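; BP_FlagZone is a flag zone that manages the flag HUD for every player.
; After a short delay on BeginPlay, it creates a WBP_Flag for each BP_Player, owned by that player's controller and added to their player screen.
; It stores the widgets in FlagRef, and its custom events relay progress bar fades, team color changes and cooldown warning text to all of them.
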(event EventFadein
  ;[1 1 1] Fade In
  (for _array_element (Variables|Default|GetFlagRef)
    (Default|PrgBarFadein _array_element)))

(event EventBeginPlay
  ;[1 1 1] Create FlagZone widget
  (Utilities|FlowControl|Delay 1.0)
  (bind _outactors (Actor|GetAllActorsOfClass "/Game/Player/BP_Player.BP_Player_C"))
  (for _array_element _outactors
    (bind _returnvalue (UserInterface|CreateWidget "/Game/HUD/WBP_Flag.WBP_Flag_C" (Game|GetPlayerController (Variables|/Script/DeathRocket_TPS.MyPlayer|GetplayerIndex _array_element))))
    (Utilities|Array|Add (Variables|Default|GetFlagRef) _returnvalue)
    (UserInterface|Viewport|AddtoPlayerScreen _returnvalue)))

(event EventFadeOut
  ;[1 1 1] Fade Out
  (for _array_element (Variables|Default|GetFlagRef)
    (Default|PrgBarFadeOut _array_element)))

(event EventBothTeamonPoint
  ;[1 1 1] Color change
  (for _array_element (Variables|Default|GetFlagRef)
    (Default|SetColorPrgBarTeam _array_element)))

(event EventUpdateWarningMessage
  ;[1 1 1] Warning Text
  (for _array_element (Variables|Default|GetFlagRef)
    (Default|SetWarningText _array_element (Variables|Default|GetbIsOnCoolDown))))

(fn ConstructionScript)